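; GameLogic is a coordinator Blueprint that tracks the score and manages the current ChildPaper page.
; It forwards assigned monster numbers to that page's CompareMonster.
; It caches the page and its transform, and replaces a page by destroying it and spawning a new ChildPaper at that transform.
; Score resets to zero in the construction script and increments through its own event.
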(event `AssignMonster`
  (params (MonsterNumber :type Integer))
  (bind _aschild_paper (cast `/Game/Game/Blueprints/ChildPaper` (`self.Childpage`)))
  (`/Game/Game/Blueprints/ChildPaper.CompareMonster` _aschild_paper MonsterNumber))

(event `ChildPaper Created`
  (params (Actor :type "Actor Object Reference"))
  (bind _output_get (set `self.Childpage` (stale `NewChildPage` _returnvalue) :!label _label))
  (set `self.ChildpageTrans` (`self.GetTransform` _output_get)))

(event `Score++`
  (`/Engine/EditorBlueprintResources/StandardMacros.IncrementInt` (`self.Score`)))

(event `NewChildPage`
  (params (CurrentChildPage :type "Actor Object Reference"))
  (`self.K2_DestroyActor` CurrentChildPage)
  (bind _returnvalue (`|SpawnActorFromClass` "/Game/Game/Blueprints/ChildPaper.ChildPaper_C" (`self.ChildpageTrans`) "Undefined" "OverrideRootScale"))
  (goto _label))

(fn `UserConstructionScript`
  (set `self.Score` 0))