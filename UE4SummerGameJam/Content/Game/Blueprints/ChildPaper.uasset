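; ChildPaper is a Blueprint for a child page that can be matched against a monster to score.
; On construction it registers itself with the GameLogic game mode and rolls one of three random child types; the switch on that type has no branches wired.
; CompareMonster checks a monster number against the type, scores through GameLogic on a match, and requests a new child page from GameLogic whatever the result.
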(event `DetermineChild`
  (bind _output_get (set `self.ChildType` (`KismetMathLibrary.RandomInteger` 3)))
  (switch `int` _output_get))

(event `CompareMonster`
  (params (MonsterNum :type Integer))
  (bind _returnvalue (`GameplayStatics.GetGameMode`))
  (`/Engine/EditorBlueprintResources/StandardMacros.CompareInt` MonsterNum (`self.ChildType`)
    (:`>`
      (bind _asgame_logic (cast `/Game/Game/Blueprints/GameLogic` _returnvalue :!label _label)))
    (:`==`
      (bind _asgame_logic_2 (cast `/Game/Game/Blueprints/GameLogic` _returnvalue))
      (`/Game/Game/Blueprints/GameLogic.Score++` _asgame_logic_2))
    (:`<`
      (goto _label)))
  (`/Game/Game/Blueprints/GameLogic.NewChildPage` _asgame_logic_2 self)
  (`/Game/Game/Blueprints/GameLogic.NewChildPage` _asgame_logic self))

(fn `UserConstructionScript`
  (bind _asgame_logic (cast `/Game/Game/Blueprints/GameLogic` (`GameplayStatics.GetGameMode`)))
  (`/Game/Game/Blueprints/GameLogic.ChildPaper Created` _asgame_logic self)
  (`self.DetermineChild`))